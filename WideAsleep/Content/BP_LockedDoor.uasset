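; BP_LockedDoor is a door that the player unlocks with a key, then can open and close freely.
; On BeginPlay it caches the first-person character, whose active inventory slot and key counter gate the first OpenDoor call.
; A successful unlock consumes one key and sets AlreadyOpened, so later calls skip the check.
; A FlipFlop alternately plays and reverses a timeline that swings the door's yaw a quarter turn.
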(event `self.ReceiveBeginPlay`
  (bind _asbp_first_person_character (cast `/Game/FirstPerson/Blueprints/BP_FirstPersonCharacter` (`GameplayStatics.GetPlayerCharacter` 0)))
  (set `self.Player Ref` _asbp_first_person_character))

(event `Open Door`
  (bind _player_ref (`self.Player Ref`))
  (if (`self.AlreadyOpened?`)
    (`/Engine/EditorBlueprintResources/StandardMacros.FlipFlop` :!label _label
      (:`A`
        (bind (_direction _rotation) (`Timeline|Rotate door timeline` :!via `PlayFromStart` :!label _label_2)
          (:`Update`
            (`SceneComponent.K2_SetRelativeRotation` (`self.Door1`) (`KismetMathLibrary.MakeRotator` 0.0 0.0 (`KismetMathLibrary.Lerp` 0.0 90.0 _rotation)) false false))))
      (:`B`
        (goto _label_2 :!via `Reverse`)))
    (elif (and (== (`/Game/FirstPerson/Blueprints/BP_FirstPersonCharacter.activeInventorySlot` _player_ref) 3) (> (`/Game/FirstPerson/Blueprints/BP_FirstPersonCharacter.keyCounter` _player_ref) 0))
      (`/Engine/EditorBlueprintResources/StandardMacros.DecrementInt` (`/Game/FirstPerson/Blueprints/BP_FirstPersonCharacter.keyCounter` _player_ref)
        (:`  `
          (set `self.AlreadyOpened?` true)
          (goto _label))))))

(fn `UserConstructionScript`)