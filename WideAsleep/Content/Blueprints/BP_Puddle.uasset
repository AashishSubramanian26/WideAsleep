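; BP_Puddle is a puddle trigger actor that plays a sound when the first-person character steps into it.
; A Box overlap begin spawns the puddle cue at the actor's location, starting partway into the audio, throttled by a short cooldown based on game time.
; Entering and leaving the box also print debug strings; overlaps from other actors are ignored.
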(event `self.Box.OnComponentBeginOverlap`
  (params (OverlappedComponent :type "PrimitiveComponent Object Reference") (OtherActor :type "Actor Object Reference") (OtherComp :type "PrimitiveComponent Object Reference") (OtherBodyIndex :type Integer) (bFromSweep :type Boolean) (SweepResult :type "HitResult Structure (by ref)"))
  (cast `/Game/FirstPerson/Blueprints/BP_FirstPersonCharacter` OtherActor)
  (`KismetSystemLibrary.PrintString` "WATWR")
  (if (> (- (`KismetSystemLibrary.GetGameTimeInSeconds`) (`self.LastPuddleSoundTime`)) 0.5)
    (`GameplayStatics.SpawnSoundAtLocation` "/Game/Audio/Puddle_cue.Puddle_cue" (`self.K2_GetActorLocation`) (struct) 1.0 1.0 4.5 null null)
    (set `self.LastPuddleSoundTime` (`KismetSystemLibrary.GetGameTimeInSeconds`))))

(event `self.Box.OnComponentEndOverlap`
  (params (OverlappedComponent :type "PrimitiveComponent Object Reference") (OtherActor :type "Actor Object Reference") (OtherComp :type "PrimitiveComponent Object Reference") (OtherBodyIndex :type Integer))
  (cast `/Game/FirstPerson/Blueprints/BP_FirstPersonCharacter` OtherActor)
  (`KismetSystemLibrary.PrintString` "OUT"))

(fn `UserConstructionScript`)