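; Brother enemy boss that runs BT_BrotherEnemy and opens the LevelWin level when its Lives run out and it dies.
; BP_Ball overlaps or Box hits cost a life, mark the player as spotted and show a blindfold at low lives.
; A Box hit leaving four lives sets blackboard MidDrink, and overlapping BP_Sink then plays a drink that restores lives.
; Tick triggers close-range headbutts or hurricane kicks, applying damage as the montage starts.
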(event `self.ReceiveActorBeginOverlap`
  (params (OtherActor :type "Actor Object Reference"))
  (bind _returnvalue (`AIBlueprintHelperLibrary.GetBlackboard` (`AIBlueprintHelperLibrary.GetAIController` self)))
  (bind _returnvalue_2 (`AIBlueprintHelperLibrary.GetBlackboard` (`AIBlueprintHelperLibrary.GetAIController` self)))
  (bind _asbp_sink (cast `/Game/Sink/BP_Sink` OtherActor)
    (:`then`
      (if (`BlackboardComponent.GetValueAsBool` _returnvalue "MidDrink")
        (`|PlayMontage` (`self.Mesh`) "/Game/BrotherEnemy/AnimationSequences/MN_Drink.MN_Drink" 0.2
          (:`OnCompleted`
            (`BlackboardComponent.SetValueAsBool` _returnvalue "MidDrink" false)
            (set `self.Lives` 6)
            (`SceneComponent.SetVisibility` (`self.Blindfold`) false false)))))
    (:`CastFailed`
      (cast `/Game/FirstPerson/Blueprints/Items/Baseball/BP_Ball` OtherActor)
      (if (> (`self.Lives`) 0)
        (`KismetSystemLibrary.PrintString` "hit by ball")
        (`|PlayMontage` (`self.Mesh`) "/Game/BrotherEnemy/AnimationSequences/MN_Flinch.MN_Flinch" 2.0
          (:`then`
            (bind _output_get (set `self.Lives` (- (`self.Lives`) 1)))
            (`BlackboardComponent.SetValueAsBool` _returnvalue_2 "MidDrink" false)
            (`BlackboardComponent.SetValueAsBool` _returnvalue_2 "HasSpottedPlayer" true)
            (if (< _output_get 5)
              (`SceneComponent.SetVisibility` (`self.Blindfold`) true false))))))))

(event `self.ReceiveBeginPlay`
  (set `self.Lives` 6)
  (set `self.MidDrink` false)
  (`AIController.RunBehaviorTree` (`AIBlueprintHelperLibrary.GetAIController` self) "/Game/BrotherEnemy/BehaviorTrees/BT_BrotherEnemy.BT_BrotherEnemy"))

(event `self.ReceiveTick`
  (params (DeltaSeconds :type "Float (single-precision)"))
  (bind _mesh (`self.Mesh`))
  (bind _returnvalue (`self.GetDistanceTo` (`GameplayStatics.GetPlayerPawn` 0)))
  (bind _returnvalue_2 (`AIBlueprintHelperLibrary.GetBlackboard` (`AIBlueprintHelperLibrary.GetAIController` self)))
  (if (<= (`self.Lives`) 0)
    (if (not (`self.isDead`))
      (set `self.isDead` true)
      (`SkeletalMeshComponent.PlayAnimation` (`self.Mesh`) "/Game/BrotherEnemy/AnimationSequences/Death.Death" false)
      (`KismetSystemLibrary.Delay` 2.6)
      (`self.K2_DestroyActor`)
      (`GameplayStatics.OpenLevel` "LevelWin"))
    (elif (`BlackboardComponent.GetValueAsBool` _returnvalue_2 "HasSpottedPlayer")
      (if (`BlackboardComponent.GetValueAsBool` _returnvalue_2 "MidDrink")
        _
        (elif (< _returnvalue 300.0)
          (if (< _returnvalue 200.0)
            (`|PlayMontage` _mesh "/Game/BrotherEnemy/AnimationSequences/MN_Headbutt.MN_Headbutt"
              (:`then`
                _))
            (else
              (`|PlayMontage` _mesh "/Game/BrotherEnemy/AnimationSequences/MN_HurricaneKick.MN_HurricaneKick"
                (:`then`
                  _))))
          (`MovementComponent.StopMovementImmediately` (`self.CharacterMovement`))
          (`GameplayStatics.ApplyDamage` (`GameplayStatics.GetPlayerPawn` 0) 20.0 null self))))))

(event `self.Box.OnComponentHit`
  (params (HitComponent :type "PrimitiveComponent Object Reference") (OtherActor :type "Actor Object Reference") (OtherComp :type "PrimitiveComponent Object Reference") (NormalImpulse :type "Vector Structure") (Hit :type "HitResult Structure (by ref)"))
  (bind _returnvalue (`AIBlueprintHelperLibrary.GetBlackboard` (`AIBlueprintHelperLibrary.GetAIController` self)))
  (bind _returnvalue_2 (`AIBlueprintHelperLibrary.GetBlackboard` (`AIBlueprintHelperLibrary.GetAIController` self)))
  (if (> (`self.Lives`) 0)
    (cast `/Game/FirstPerson/Blueprints/Items/Baseball/BP_Ball` OtherActor)
    (`KismetSystemLibrary.PrintString` "hit by ball")
    (`|PlayMontage` (`self.Mesh`) "/Game/BrotherEnemy/AnimationSequences/MN_Flinch.MN_Flinch" 2.0
      (:`then`
        (bind _output_get (set `self.Lives` (- (`self.Lives`) 1)))
        (`BlackboardComponent.SetValueAsBool` _returnvalue_2 "MidDrink" false)
        (`BlackboardComponent.SetValueAsBool` _returnvalue_2 "HasSpottedPlayer" true)
        (if (< _output_get 5)
          (`SceneComponent.SetVisibility` (`self.Blindfold`) true false)
          (if (== _output_get 4)
            (`BlackboardComponent.SetValueAsBool` _returnvalue "MidDrink" true)
            (`KismetSystemLibrary.PrintString` "should start moving to sink")
            (`KismetSystemLibrary.PrintString` (`KismetStringLibrary.Conv_BoolToString` (`BlackboardComponent.GetValueAsBool` _returnvalue "MidDrink")))))))))

(fn `UserConstructionScript`)