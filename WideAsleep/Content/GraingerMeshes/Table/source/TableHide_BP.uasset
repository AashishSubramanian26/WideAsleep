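; Table hiding spot that lets the first-person player hide and look around through the table's own camera.
; Overlapping the box enables input and opens a gate so the hide action toggles the player's Hide/Unhide; leaving closes the gate.
; Hiding blends the view to this actor and starts a self-recalling short-delay loop that applies clamped look input to the camera.
; When not hidden, look input passes through to the player.
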(event `self.ReceiveBeginPlay`
  (bind _asbp_first_person_character (cast `/Game/FirstPerson/Blueprints/BP_FirstPersonCharacter` (`GameplayStatics.GetPlayerCharacter` 0)))
  (set `self.Player Reference` _asbp_first_person_character))

(event `EnhancedInput|/Game/Input/IA_Hide`
  (params (ActionValue :type Boolean) (ElapsedSeconds :type "Float (double-precision)") (TriggeredSeconds :type "Float (double-precision)") (InputAction :type "InputAction Object Reference" :default "/Game/Input/IA_Hide.IA_Hide"))
  (bind _player_reference (`self.Player Reference`))
  (:`Started`
    (`/Engine/EditorBlueprintResources/StandardMacros.Gate` false :!label _label
      (:`Exit`
        ;[1 1 1] If we are hiding, need to unhide and vise versa
        (if (`/Game/FirstPerson/Blueprints/BP_FirstPersonCharacter.isHiding?` _player_reference)
          (`/Game/FirstPerson/Blueprints/BP_FirstPersonCharacter.Unhide` _player_reference)
          (else
            (`/Game/FirstPerson/Blueprints/BP_FirstPersonCharacter.Hide` _player_reference)
            (`|ExecutionSequence`
              (:`then_0`
                (`PlayerController.SetViewTargetWithBlend` (`GameplayStatics.GetPlayerController` 0) self 0.5 "VTBlend_Linear" 0.0 false)
                (`self.Move Camera`))
              (:`then_1`
                (`KismetSystemLibrary.Delay` 0.2)
                (`self.EnableInput` (`GameplayStatics.GetPlayerController` 0) :!label _label_2)
                (goto _label :!via `Open`)))))))))

(event `self.Box.OnComponentBeginOverlap`
  (params (OverlappedComponent :type "PrimitiveComponent Object Reference") (OtherActor :type "Actor Object Reference") (OtherComp :type "PrimitiveComponent Object Reference") (OtherBodyIndex :type Integer) (bFromSweep :type Boolean) (SweepResult :type "HitResult Structure (by ref)"))
  (bind _asbp_first_person_character (cast `/Game/FirstPerson/Blueprints/BP_FirstPersonCharacter` OtherActor))
  (set `self.Player Reference` _asbp_first_person_character)
  (goto _label_2))

(event `self.Box.OnComponentEndOverlap`
  (params (OverlappedComponent :type "PrimitiveComponent Object Reference") (OtherActor :type "Actor Object Reference") (OtherComp :type "PrimitiveComponent Object Reference") (OtherBodyIndex :type Integer))
  (cast `/Game/FirstPerson/Blueprints/BP_FirstPersonCharacter` OtherActor)
  (`self.EnableInput` (`GameplayStatics.GetPlayerController` 0))
  (goto _label :!via `Close`))

(event `Move Camera`
  (if (`/Game/FirstPerson/Blueprints/BP_FirstPersonCharacter.isHiding?` (`self.Player Reference`))
    (`SceneComponent.K2_SetRelativeRotation` (`self.Camera`) (`KismetMathLibrary.MakeRotator` 0.0 (* (stale `InputAxis|LookUp` _output_get_2) -1.0) (stale `InputAxis|Turn` _output_get_2)) false false)
    (`KismetSystemLibrary.Delay` 0.001)
    (`self.Move Camera`)))

(event `InputAxis|LookUp`
  (params (AxisValue :type "Float (single-precision)"))
  (bind _player_reference (`self.Player Reference`))
  (if (`/Game/FirstPerson/Blueprints/BP_FirstPersonCharacter.isHiding?` _player_reference)
    (bind _output_get (set `self.Pitch` (+ (`self.Pitch`) AxisValue)))
    (bind _output_get_2 (set `self.Pitch` (`KismetMathLibrary.FClamp` _output_get -20.0 20.0)))
    (else
      (`Pawn.AddControllerPitchInput` _player_reference AxisValue))))

(event `InputAxis|Turn`
  (params (AxisValue :type "Float (single-precision)"))
  (bind _player_reference (`self.Player Reference`))
  (if (`/Game/FirstPerson/Blueprints/BP_FirstPersonCharacter.isHiding?` _player_reference)
    (bind _output_get (set `self.Yaw` (+ (`self.Yaw`) AxisValue)))
    (bind _output_get_2 (set `self.Yaw` (`KismetMathLibrary.FClamp` _output_get -60.0 60.0)))
    (else
      (`Pawn.AddControllerYawInput` _player_reference AxisValue))))

(fn `UserConstructionScript`)